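; Player character Blueprint with first- and third-person gun meshes and a sprint action.
; BeginPlay sets game-only input, hides the cursor, attaches two first-person gun slots and a third-person gun to hand sockets, then forces both slots visible to work around a follow bug.
; Sprint press and release change walk speed locally, then call Rep-prefixed events that apply the same speeds, apparently for network replication.
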(event `self.ReceiveBeginPlay`
  (bind _returnvalue (`GameplayStatics.GetPlayerController` 0))
  (`WidgetBlueprintLibrary.SetInputMode_GameOnly` _returnvalue)
  (set `PlayerController.bShowMouseCursor` false _returnvalue)
  (`SceneComponent.K2_AttachToComponent` (`self.FirstPersonGunActorSlot1`) (`self.FirstPersonMesh`) "hand_rSocket" "SnapToTarget" "KeepWorld" "KeepWorld" false)
  (`SceneComponent.K2_AttachToComponent` (`self.ThirdPersonGunMesh`) (`self.Mesh`) "hand_rSocket" "SnapToTarget" "KeepWorld" "KeepWorld" true)
  (`SceneComponent.K2_AttachToComponent` (`self.FirstPersonGunActorSlot2`) (`self.FirstPersonMesh`) "hand_rSocket" "SnapToTarget" "KeepWorld" "KeepWorld" true)
  ;[1 1 1] Fixes weird follow bug somehow (??)
  (`SceneComponent.SetVisibility` (`self.FirstPersonGunActorSlot1`) true true)
  (`SceneComponent.SetVisibility` (`self.FirstPersonGunActorSlot2`) true true))

(event `self.ReceiveTick`
  (params (DeltaSeconds :type "Float (single-precision)")))

(event `InputAction|Sprint`
  (params (Key :type "Key Structure"))
  (bind _charactermovement (`self.CharacterMovement`))
  (:`Pressed`
    (set `CharacterMovementComponent.MaxWalkSpeed` 800.0 _charactermovement)
    (`self.Rep_SprintingStart`))
  (:`Released`
    (set `CharacterMovementComponent.MaxWalkSpeed` 600.0 _charactermovement)
    (`self.RepSprintingEnd`)))

(event `Rep_SprintingStart`
  (set `CharacterMovementComponent.MaxWalkSpeed` 800.0 (`self.CharacterMovement`)))

(event `RepSprintingEnd`
  (set `CharacterMovementComponent.MaxWalkSpeed` 600.0 (`self.CharacterMovement`)))

(fn `UserConstructionScript`)